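; BP_AuraPlayerController is the player controller Blueprint, adding debug input and a camera occlusion check.
; On BeginPlay a looping timer, rather than Tick, periodically has AuraCameraFade sync the actors occluding the camera.
; Debug key E toggles the inventory menu through the inventory management component, and debug key T flip-flops global time dilation between slow motion and normal speed.
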(event Custom|检测相机遮挡
  (Class|AuraCameraFadeComponent|SyncOccludedActors (Variables|Default|GetAuraCameraFade)))

(event EventBeginPlay
  (Utilities|Time|SetTimerbyEvent (delegate Custom|检测相机遮挡) 0.1 true))

(event EventTick
  (params (DeltaSeconds :type Float%20%28single-precision%29)))

(event Input|KeyboardEvents|DebugKeyE
  (params (Key :type Key%20Structure :default "None") (ActionValue :type Input%20Action%20Value%20Structure))
  ;[0.15 0.15 0.15 0.5] 测试用
  (:Pressed
    (Class|InvInventoryComponent|ToggleInventoryMenu (Variables|Default|GetBP_Inv_ManagementCompoent))))

(event Input|KeyboardEvents|DebugKeyT
  (params (Key :type Key%20Structure :default "None") (ActionValue :type Input%20Action%20Value%20Structure))
  ;[0.15 0.15 0.15 0.5] 测试用
  (:Pressed
    (Utilities|FlowControl|FlipFlop
      (:A
        (Utilities|Time|SetGlobalTimeDilation 0.1))
      (:B
        (Utilities|Time|SetGlobalTimeDilation 1.0)))))

(fn ConstructionScript)