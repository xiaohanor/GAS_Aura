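; Melee attack gameplay ability that plays a random attack montage from its avatar and damages living players near the hit point.
; It waits for the montage's gameplay event tag, then finds the matching combat socket location and runs a small radius query there that ignores itself.
; Each target found takes damage through CauseDamage.
; The ability ends after the hit, when the montage finishes or is interrupted, or when no montages exist.
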(event Ability|EventActivateAbility
  (bind _returnvalue (Ability|GetAvatarActorfromActorInfo))
  (bind _returnvalue_2 (Class|CombatInterface|GetAttackMontages(Message) (Ability|GetAvatarActorfromActorInfo)))
  (if (Utilities|Array|IsNotEmpty _returnvalue_2)
    (bind _output_get (Variables|Default|SetAttackMontages (.OutItem (Utilities|Array|Random _returnvalue_2))))
    (|PlayMontageandWaitProxy "None" (.montage _output_get) 1.0 "None" true 1.0 0.0 false
      (:then
        (Ability|Tasks|WaitGameplayEvent (.montagetag _output_get) 0
          (:EventReceived
            (bind _returnvalue_3 (Class|CombatInterface|GetCombatSocketLocation(Message) _returnvalue (.montagetag _output_get)))
            (bind _outoverlappingactors (Class|AuraAbilitySystemLibrary|GetLivePlayersWithinRadius (Utilities|Array|MakeArray _returnvalue) 5e+01 _returnvalue_3))
            (for _array_element _outoverlappingactors
              (Class|AuraDamageGameplayAbility|CauseDamage _array_element))
            (Ability|EndAbility))))
      (:OnCompleted
        (Ability|EndAbility :!label _label))
      (:OnInterrupted
        (goto _label))
      (:OnCancelled
        (goto _label)))
    (else
      (Ability|EndAbility))))

(event Ability|EventOnEndAbility
  (params (bWasCancelled :type Boolean)))