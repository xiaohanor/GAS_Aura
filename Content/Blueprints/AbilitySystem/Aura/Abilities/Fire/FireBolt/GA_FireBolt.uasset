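; GA_FireBolt is the Fire Bolt gameplay ability that casts a projectile toward the point under the mouse.
; On activation it gets target data under the cursor, turns the avatar toward the hit location and plays the cast montage.
; It waits for the montage's FireBolt gameplay event to spawn the projectile from the weapon socket, then ends after a short delay.
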(event Ability|EventActivateAbility
  (bind _datahandle (|TargetDataUnderMouse)
    (:ValidData
      (bind _output_get (Variables|Default|SetLocation (.Location (Collision|BreakHitResult (Ability|TargetData|GetHitResultfromTargetData _datahandle)))))
      (Class|CombatInterface|UpdatedFacingTarget(Message) (Ability|GetAvatarActorfromActorInfo) _output_get)
      (|PlayMontageandWaitProxy "None" "/Game/Assets/Characters/Aura/Animations/Abilities/AM_Cast_FireBolt.AM_Cast_FireBolt" 1.0 "None" true 1.0 0.0 false
        (:then
          (Ability|Tasks|WaitGameplayEvent "(TagName=\"AuraGameplayTags.Montage.FireBolt\")" 0
            (:EventReceived
              (Class|AuraGACastProjectile|SpawnProjectile (Variables|Default|GetLocation) (GameplayTags|MakeLiteralGameplayTag "(TagName=\"AuraGameplayTags.CombatSocket.Weapon\")"))
              (Utilities|FlowControl|Delay 0.2)
              (Ability|EndAbility))))))))