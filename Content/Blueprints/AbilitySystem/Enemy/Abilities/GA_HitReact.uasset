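; Enemy hit-react gameplay ability that plays the avatar's hit reaction montage.
; On activation it applies GE_HitReact to the owner and gets the montage through CombatInterface, caching the interface reference after the first cast.
; The ability ends when the montage completes, is interrupted or is cancelled, and OnEndAbility removes the effect by its stored handle.
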(event Ability|EventActivateAbility
  (bind _returnvalue (Ability|ApplyGameplayEffectToOwner "/Game/Blueprints/AbilitySystem/Enemy/Effects/GE_HitReact.GE_HitReact_C"))
  (Variables|Default|SetHitReact _returnvalue)
  (if (Utilities|IsValidInterface (Variables|Default|GetAs%20Combat%20Interface))
    _
    (else
      (bind _ascombat_interface (Utilities|Casting|CastToCombatInterface (Ability|GetAvatarActorfromActorInfo)))
      (bind _output_get (Variables|Default|SetAs%20Combat%20Interface _ascombat_interface))
      (bind _returnvalue_2 (Class|CombatInterface|GetHitReactMontage _output_get))))
  (|PlayMontageandWaitProxy "None" _returnvalue_2 1.0 "None" true 1.0 0.0 false
    (:OnCompleted
      _)
    (:OnInterrupted
      _)
    (:OnCancelled
      _))
  (Ability|EndAbility))

(event Ability|EventOnEndAbility
  (params (bWasCancelled :type Boolean))
  (Ability|RemoveGameplayEffectFromOwnerWithHandle (Variables|Default|GetHitReact)))