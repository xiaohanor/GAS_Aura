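; Enemy gameplay ability that summons random minions at a shuffled set of spawn locations.
; A macro first fires a GroundSummon gameplay cue at each location, one per tick, then the ability plays a random attack montage from the avatar.
; The montage's gameplay event starts a delay-driven loop that spawns minions one by one, slightly raised above each point.
; The graph never calls EndAbility or resets either loop index.
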(event Ability|EventActivateAbility
  (bind _returnvalue (Class|AuraGASummon|GetSpawnLocations))
  (bind _output_get (Variables|Default|SetSpawnLocations _returnvalue))
  (Utilities|Array|Shuffle _output_get)
  (|生成Cue
    (:false
      (bind _returnvalue_2 (Class|CombatInterface|GetAttackMontages(Message) (Ability|GetAvatarActorfromActorInfo)))
      (if (Utilities|Array|IsNotEmpty _returnvalue_2)
        (bind _output_get_2 (Variables|Default|SetAttackMontages (.OutItem (Utilities|Array|Random _returnvalue_2))))
        (|PlayMontageandWaitProxy "None" (.montage _output_get_2) 1.0 "None" true 1.0 0.0 false
          (:then
            (Ability|Tasks|WaitGameplayEvent (.montagetag _output_get_2) 0
              (:EventReceived
                (if (< (Variables|Default|GetSpawnLocationIndex) (Utilities|Array|Length (Variables|Default|GetSpawnLocations))) :!label _label
                  (Game|SpawnActorfromClass (Class|AuraGASummon|GetRandomMinionClasses) (Math|Transform|MakeTransform (+ (Utilities|Array|Get(acopy) (Variables|Default|GetSpawnLocations) (Variables|Default|GetSpawnLocationIndex)) "0.000000,0.000000,70.000000") "0, 0, 0" "1.000000,1.000000,1.000000") "AdjustIfPossibleButDontSpawnIfColliding" "MultiplyWithRoot" 0 0)
                  (Math|Integer|IncrementInt (Variables|Default|GetSpawnLocationIndex)
                    (:%20%20
                      (Utilities|FlowControl|Delay 0.2)
                      (goto _label))))))))))))

(event Ability|EventOnEndAbility
  (params (bWasCancelled :type Boolean)))