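; GA_EnemyFireBolt is an enemy gameplay ability that fires a projectile at the avatar's combat target.
; On activation it picks a random attack montage from the avatar, plays it and waits for that montage's gameplay event tag.
; When the event arrives, it queries the tagged socket location and spawns the projectile toward the target's location.
; The ability ends when the montage completes, is interrupted or cancelled, or immediately if no montages exist.
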(event Ability|EventActivateAbility
  (bind _returnvalue (Ability|GetAvatarActorfromActorInfo))
  (bind _returnvalue_2 (Class|CombatInterface|GetAttackMontages(Message) (Ability|GetAvatarActorfromActorInfo)))
  (if (Utilities|Array|IsNotEmpty _returnvalue_2)
    (bind _output_get (Variables|Default|SetAttackMontages (.OutItem (Utilities|Array|Random _returnvalue_2))))
    (|PlayMontageandWaitProxy "None" (.montage _output_get) 1.0 "None" true 1.0 0.0 false
      (:then
        (Ability|Tasks|WaitGameplayEvent (.montagetag _output_get) 0
          (:EventReceived
            (Class|CombatInterface|GetCombatSocketLocation(Message) _returnvalue (.sockettag _output_get))
            (bind _returnvalue_3 (Class|EnemyInterface|GetCombatTarget(Message) _returnvalue))
            (Class|AuraGACastProjectile|SpawnProjectile (Transformation|GetActorLocation _returnvalue_3)))))
      (:OnCompleted
        (Ability|EndAbility :!label _label))
      (:OnInterrupted
        (goto _label))
      (:OnCancelled
        (goto _label)))
    (else
      (Ability|EndAbility))))

(event Ability|EventOnEndAbility
  (params (bWasCancelled :type Boolean)))