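; GA_MeleeAttack is an enemy melee ability that plays a random attack montage from the avatar and damages nearby live players.
; The montage's gameplay event triggers a small sphere query at the matching combat socket, excluding the avatar.
; Each player found takes damage and spawns their own blood effect, with an impact sound on a hit.
; The ability ends on a miss or when the montage completes or is interrupted.
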(event Ability|EventActivateAbility
  (bind _returnvalue (Ability|GetAvatarActorfromActorInfo))
  (bind _returnvalue_2 (Class|CombatInterface|GetAttackMontages(Message) (Ability|GetAvatarActorfromActorInfo)))
  (if (Utilities|Array|IsNotEmpty _returnvalue_2)
    (bind _output_get (Variables|Default|SetAttackMontages (.OutItem (Utilities|Array|Random _returnvalue_2))))
    (|PlayMontageandWaitProxy "None" (.montage _output_get) 1.0 "None" true 1.0 0.0 false
      (:then
        (Ability|Tasks|WaitGameplayEvent (.montagetag _output_get) 0
          (:EventReceived
            (bind _returnvalue_3 (Class|CombatInterface|GetCombatSocketLocation(Message) _returnvalue (.montagetag _output_get)))
            (bind _output_get_2 (Variables|Default|SetSocketLocation _returnvalue_3))
            (bind _outoverlappingactors (Class|AuraAbilitySystemLibrary|GetLivePlayersWithinRadius (Utilities|Array|MakeArray _returnvalue) 5e+01 _output_get_2))
            (for _array_element _outoverlappingactors
              (Class|AuraDamageGameplayAbility|CauseDamage _array_element)
              (Variables|Default|SetHasHitTarget true)
              (bind _returnvalue_4 (Class|CombatInterface|GetBloodEffect(Message) _array_element))
              (Niagara|SpawnSystematLocation _returnvalue_4 (Variables|Default|GetSocketLocation)))
            (if (Variables|Default|GetHasHitTarget)
              (Audio|PlaySoundatLocation (.ImpactSound (Utilities|Struct|BreakTaggedMontage (Variables|Default|GetAttackMontages))) (Variables|Default|GetSocketLocation) "0, 0, 0" 1.0 1.0 0.0 0 0 0 0)
              (else
                (Ability|EndAbility))))))
      (:OnCompleted
        (Ability|EndAbility :!label _label))
      (:OnInterrupted
        (goto _label))
      (:OnCancelled
        (goto _label)))
    (else
      (Ability|EndAbility))))

(event Ability|EventOnEndAbility
  (params (bWasCancelled :type Boolean)))